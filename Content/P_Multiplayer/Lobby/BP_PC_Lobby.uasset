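; Player controller for the multiplayer lobby that shows the lobby menu and manages the player's info and ready status.
; On BeginPlay, the local controller creates WBP_LobbyMenu, enables the cursor with Game and UI input, then reports its info.
; ROS-prefixed events pass the controller to BP_LobbyGameMode, with the ready toggle first flipping Ready in PlayerInfo.
; UpdatePlayerInfo repeats the report after a short delay.
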(event Custom|Update%20Player%20Info
  (Utilities|FlowControl|Delay 0.1)
  (CallFunction|ROSUpdatePlayerInfo))

(event Custom|ROS_Update%20Player%20Info
  (bind _asbp_lobby_game_mode (Utilities|Casting|CastToBP_LobbyGameMode (Game|GetGameMode)))
  (Default|UpdatePlayerInfo _asbp_lobby_game_mode self))

(event Custom|ROS_ToggelReadyStatus
  (bind _player_info (Variables|Default|GetPlayer%20Info))
  (Utilities|Struct|SetmembersinS_PlayerInfo _player_info (not (.Ready? (Utilities|Struct|BreakS_PlayerInfo _player_info))))
  (bind _asbp_lobby_game_mode (Utilities|Casting|CastToBP_LobbyGameMode (Game|GetGameMode)))
  (Default|UpdatePlayerInfo _asbp_lobby_game_mode self))

(event EventBeginPlay
  (if (Pawn|IsLocalPlayerController)
    (bind _returnvalue (UserInterface|CreateWidget "/Game/P_Menu/Widgets/WBP_LobbyMenu.WBP_LobbyMenu_C"))
    (Variables|Default|SetLobby%20UI _returnvalue)
    (UserInterface|Viewport|AddtoViewport _returnvalue 0)
    (Variables|Default|SetbShowMouseCursor true)
    (Input|SetInputModeGameandUI self _returnvalue "DoNotLock" true false)
    (CallFunction|ROSUpdatePlayerInfo)))

(fn ConstructionScript)